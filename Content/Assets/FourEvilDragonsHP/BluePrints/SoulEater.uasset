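; SoulEater is a boss Blueprint for a side-scroller, built on a parent class whose BeginPlay and Death logic it extends.
; On BeginPlay it sets its boss name, fills its health and registers itself as the current boss reference on the SideScrollerGameMode.
; On Death it runs the parent logic, then plays a non-looping animation on its skeletal mesh.
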(event EventBeginPlay
  (|CallParentFunction)
  ;[1 1 1] initialization
  (Variables|Default|SetBossName "SoulEater")
  (Variables|Default|SetBossHealth (Variables|Default|GetFullHealth))
  (bind _asside_scroller_game_mode (Utilities|Casting|CastToSideScrollerGameMode (Game|GetGameMode)))
  (Variables|/Game/SideScrollerBP/Blueprints/SideScrollerGameMode.SideScrollerGameMode_C|SetCurrentBossReference _asside_scroller_game_mode self))

(event Collision|EventActorBeginOverlap
  (params (OtherActor :type Actor%20Object%20Reference))
  (|CallParentFunction OtherActor) ; 此节点被禁用，将不会被调用。\n从引脚连出引线来编译功能。
)

(event EventTick
  (params (DeltaSeconds :type Float%20%28single-precision%29))
  (|CallParentFunction DeltaSeconds) ; 此节点被禁用，将不会被调用。\n从引脚连出引线来编译功能。
)

(fn ConstructionScript
  (|CallParentFunction))

(fn Death
  (|CallParentFunction)
  (Components|Animation|PlayAnimation (Variables|Default|GetSkeletalMesh) 0 false))